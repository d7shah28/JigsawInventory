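; BP_MasterItemObject is an item data object with a footprint, icon and item class, apparently for a grid-style inventory.
; Rotate toggles a single IsRotated flag, which drives the dimension and icon getters.
; When rotated, GetDimensions swaps X and Y and GetIcon returns a separate rotated icon, leaving the stored values untouched.
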(fn GetDimensions
  (bind _dimensions (Variables|Private|GetDimensions))
  (if (Variables|Private|GetisRotated?)
    (return (Utilities|Struct|MakeIntPoint (.y _dimensions) (.x _dimensions)))
    (else
      (return (Variables|Private|GetDimensions)))))

(fn GetIcon
  (return (select (Variables|Private|GetisRotated?) (Variables|Private|GetIconRotated) (Variables|Private|GetIcon))))

(fn GetItemClass
  (return (Variables|Private|GetItemClass)))

(fn Rotate
  (Variables|Private|SetisRotated? (not (Variables|Private|GetisRotated?))))

(fn IsRotated
  (return (Variables|Private|GetisRotated?)))